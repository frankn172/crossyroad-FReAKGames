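; BP_Car is a traffic vehicle that drives along the Y axis and jumps back to its anchor when it passes either bound.
; The construction script randomly picks a car or one of two trucks and a signed speed, adjusting height and rotation by type.
; Positive speeds move the anchor to a fixed Y start and reorient the mesh.
; Tick adds Speed per frame without delta-time scaling; the zero-speed reroll is unconnected.
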(event EventBeginPlay)

(event Collision|EventActorBeginOverlap
  (params (OtherActor :type Actor%20Object%20Reference)))

(event EventTick
  (params (DeltaSeconds :type Float%20%28single-precision%29))
  (bind _returnvalue (Transformation|GetActorLocation))
  (Transformation|SetActorLocation (+ (Transformation|GetActorLocation) (Math|Vector|MakeVector 0.0 (Variables|Default|GetSpeed) 0.0)) false false)
  (if (or (< (.y _returnvalue) -1.3e+03) (> (.y _returnvalue) 1.3e+03))
    (Transformation|SetActorLocation (Variables|Default|GetAnchor) false false)
    (else
      (Utilities|FlowControl|MultiGate false false -1))))

(fn ConstructionScript
  (Variables|Default|SetAnchor (Transformation|GetActorLocation))
  (bind _output_get (Variables|Default|SetCar%20Type (Math|Random|RandomInteger 3)))
  (switch int _output_get
    (:0
      (Components|StaticMesh|SetStaticMesh (Variables|Default|GetStaticMesh) "/Game/Meshes/car1.car1"))
    (:1
      (Components|StaticMesh|SetStaticMesh (Variables|Default|GetStaticMesh) "/Game/Meshes/Red_Truck.Red_Truck")
      (bind _output_get_2 (Variables|Default|SetAnchor (Math|Vector|MakeVector (.x (Variables|Default|GetAnchor)) (.y (Variables|Default|GetAnchor)) 2.4e+02) :!label _label))
      (Transformation|SetActorLocationAndRotation _output_get_2 "0,180.000000, 0"))
    (:2
      (Components|StaticMesh|SetStaticMesh (Variables|Default|GetStaticMesh) "/Game/Meshes/Rocket_Truck.Rocket_Truck")
      (goto _label)))
  (CallFunction|RandomizeSpeed)
  (if (> (Variables|Default|GetSpeed) 0.0)
    (switch int (Variables|Default|GetCar%20Type)
      (:0
        (Variables|Default|SetAnchor (Math|Vector|MakeVector (.x (Variables|Default|GetAnchor)) -9e+02 (.z (Variables|Default|GetAnchor))))
        (Transformation|SetActorRotation "0,-90.000000, 0"))
      (:1
        (Variables|Default|SetAnchor (Math|Vector|MakeVector (.x (Variables|Default|GetAnchor)) -9e+02 (.z (Variables|Default|GetAnchor))) :!label _label_2)
        (Transformation|SetActorRotation "0,0.000000, 0"))
      (:2
        (goto _label_2)))))

(fn RandomizeSpeed
  (bind _output_get (Variables|Default|SetSpeed (Math|Random|RandomFloatinRange -3e+01 3e+01))))