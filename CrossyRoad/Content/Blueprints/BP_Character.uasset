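; Character Blueprint that moves by directional hops in four directions, each bound to its own input action.
; Pressing an action snaps the mesh rotation for that direction, and releasing it adds a fixed world-axis launch with upward lift.
; JumpCounter caps launches at MaxJumps until landing resets it.
; Only the right-jump press checks and sets InAir to block re-rotation, and landing clears that flag.
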(event EventBeginPlay)

(event EventTick
  (params (DeltaSeconds :type Float%20%28single-precision%29)))

(event EventOnLanded
  (params (Hit :type Hit%20Result%20Structure%20%28by%20ref%29))
  (Variables|Default|SetJump_counter 0.0)
  (Variables|Default|SetIn%20Air false))

(event Input|ActionEvents|InputActionActionJumpingUp
  (params (Key :type Key%20Structure :default "None"))
  (:Pressed
    (Transformation|SetRelativeRotation (Variables|Character|GetMesh) "360.000000,0.000000,270.000000" false false))
  (:Released
    (if (< (Variables|Default|GetJump_counter) (Variables|Default|GetMax_Jumps))
      (Variables|Default|SetJump_counter (+ (Variables|Default|GetJump_counter) 1.0))
      (Character|LaunchCharacter "200.000000,0.000000,200.000000" false false))))

(event Input|ActionEvents|InputActionActionJumpDown
  (params (Key :type Key%20Structure :default "None"))
  (:Pressed
    (Transformation|SetRelativeRotation (Variables|Character|GetMesh) "180.000000, 0,90.000000" false false))
  (:Released
    (if (< (Variables|Default|GetJump_counter) (Variables|Default|GetMax_Jumps))
      (Variables|Default|SetJump_counter (+ (Variables|Default|GetJump_counter) 1.0))
      (Character|LaunchCharacter "-200.000000,0.000000,200.000000" false false))))

(event Input|ActionEvents|InputActionActionJumpLeft
  (params (Key :type Key%20Structure :default "None"))
  (:Pressed
    (Transformation|SetRelativeRotation (Variables|Character|GetMesh) "0.000000,-90.000000,-90.000000" false false))
  (:Released
    (if (< (Variables|Default|GetJump_counter) (Variables|Default|GetMax_Jumps))
      (Variables|Default|SetJump_counter (+ (Variables|Default|GetJump_counter) 1.0))
      (Character|LaunchCharacter "0.000000,-200.000000,200.000000" false false))))

(event Input|ActionEvents|InputActionActionJumpRight
  (params (Key :type Key%20Structure :default "None"))
  (:Pressed
    (if (not (Variables|Default|GetIn%20Air))
      (Transformation|SetRelativeRotation (Variables|Character|GetMesh) "0.000000,90.000000,-90.000000" false false)
      (Variables|Default|SetIn%20Air true)))
  (:Released
    (if (< (Variables|Default|GetJump_counter) (Variables|Default|GetMax_Jumps))
      (Variables|Default|SetJump_counter (+ (Variables|Default|GetJump_counter) 1.0))
      (Character|LaunchCharacter "0.000000,200.000000,200.000000" false false))))

(fn ConstructionScript)