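; BP_Lane is a lane tile actor for what looks like an endless crossing level.
; When the player overlaps its trigger, it asks the LaneSpawner for a new lane with its dark flag and a random lane number, then destroys itself.
; RandomizeLane picks a grass, rail, river or road mesh, and SpawnObjects spawns a BP_Car for lane type 1.
; The vehicle speed and reset logic is disconnected.
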(event OnComponentBeginOverlap(TriggerPoint)
  (params (OverlappedComponent :type Primitive%20Component%20Object%20Reference) (OtherActor :type Actor%20Object%20Reference) (OtherComp :type Primitive%20Component%20Object%20Reference) (OtherBodyIndex :type Integer) (bFromSweep :type Boolean) (SweepResult :type Hit%20Result%20Structure%20%28by%20ref%29))
  (Utilities|Casting|CastToBP_Player OtherActor)
  (Default|SpawnLaneatSpawnPoint (Variables|Components|GetLaneSpawner) (Variables|Default|GetisDark) (Math|Random|RandomInteger 3))
  (Actor|DestroyActor))

(event EventBeginPlay)

(event Collision|EventActorBeginOverlap
  (params (OtherActor :type Actor%20Object%20Reference)))

(event EventTick
  (params (DeltaSeconds :type Float%20%28single-precision%29)))

(fn ConstructionScript)

(fn RandomizeLane
  (Components|StaticMesh|SetStaticMesh (Variables|Debug|GetStaticMeshComponent) (Utilities|Select :Index (Math|Random|RandomIntegerinRange 0 3) :Option%200 "/Game/Meshes/grass_tile_dark.grass_tile_dark" :Option%201 "/Game/Meshes/rail.rail" :Option%202 "/Game/Meshes/river_tile.river_tile" :Option%203 "/Game/Meshes/road_edge.road_edge")))

(fn SpawnObjects
  (switch int (Variables|Default|GetLaneType)
    (:1
      (bind _returnvalue (Game|SpawnActorfromClass "/Game/Blueprints/BP_Car.BP_Car_C" (Math|Transform|MakeTransform (- (Transformation|GetWorldLocation (Variables|Default|GetSpawnPoint)) "0.000000,-500.000000,200.000000") "0,-90.000000, 0" "3.000000,3.000000,3.000000") "Undefined" 0 0))
      (Variables|Default|SetVehicle _returnvalue))))