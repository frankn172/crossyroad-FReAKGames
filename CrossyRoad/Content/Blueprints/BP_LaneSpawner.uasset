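; Lane spawner actor that builds a chain of BP_Lane tiles of grass, road or river type.
; On BeginPlay it lays a short starting run of grass lanes, the first placed relative to the player pawn.
; Each later lane spawns at the newest lane's SpawnPoint, with grass alternating between light and dark meshes.
; SpawnLane sets mesh and type, hands the lane a spawner reference, then calls its SpawnObjects.
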(event EventBeginPlay
  (CallFunction|SpawnInitialLanes))

(event Collision|EventActorBeginOverlap
  (params (OtherActor :type Actor%20Object%20Reference)))

(event EventTick
  (params (DeltaSeconds :type Float%20%28single-precision%29)))

(fn ConstructionScript)

(fn SpawnLane
  (params (SpawnLocation :type Vector) (isDark :type Boolean) (LaneType :type Integer))
  (bind _returnvalue (Game|SpawnActorfromClass "/Game/Blueprints/BP_Lane.BP_Lane_C" (Math|Transform|MakeTransform (+ SpawnLocation (Math|Vector|MakeVector 4e+01 0.0 0.0)) "0, 0, 0" "1,1,1") "Undefined" 0 0))
  (bind _output_get (Variables|Default|SetNewestLane _returnvalue))
  (Variables|/Game/Blueprints/BP_Lane.BP_Lane_C|SetLaneSpawner _output_get self)
  (switch int LaneType
    (:0
      (if isDark
        (Components|StaticMesh|SetStaticMesh (Variables|/Script/Engine.StaticMeshActor|GetStaticMeshComponent (Variables|Default|GetNewestLane)) "/Game/Meshes/grass_tile_light.grass_tile_light")
        (Variables|/Game/Blueprints/BP_Lane.BP_Lane_C|SetisDark (Variables|Default|GetNewestLane) false)
        (else
          (Components|StaticMesh|SetStaticMesh (Variables|/Script/Engine.StaticMeshActor|GetStaticMeshComponent (Variables|Default|GetNewestLane)) "/Game/Meshes/grass_tile_dark.grass_tile_dark")
          (Variables|/Game/Blueprints/BP_Lane.BP_Lane_C|SetisDark (Variables|Default|GetNewestLane) true)))
      (Variables|/Game/Blueprints/BP_Lane.BP_Lane_C|SetLaneType (Variables|Default|GetNewestLane) 0))
    (:1
      (Components|StaticMesh|SetStaticMesh (Variables|/Script/Engine.StaticMeshActor|GetStaticMeshComponent (Variables|Default|GetNewestLane)) "/Game/Meshes/road_edge.road_edge")
      (Variables|/Game/Blueprints/BP_Lane.BP_Lane_C|SetLaneType (Variables|Default|GetNewestLane) 1))
    (:2
      (Components|StaticMesh|SetStaticMesh (Variables|/Script/Engine.StaticMeshActor|GetStaticMeshComponent (Variables|Default|GetNewestLane)) "/Game/Meshes/river_tile.river_tile")
      (Variables|/Game/Blueprints/BP_Lane.BP_Lane_C|SetLaneType (Variables|Default|GetNewestLane) 2))
    (:3
      (Components|StaticMesh|SetStaticMesh (Variables|/Script/Engine.StaticMeshActor|GetStaticMeshComponent (Variables|Default|GetNewestLane)) "/Game/Meshes/road_edge.road_edge")
      (Variables|/Game/Blueprints/BP_Lane.BP_Lane_C|SetLaneType (Variables|Default|GetNewestLane) 3)))
  (Default|SpawnObjects (Variables|Default|GetNewestLane)))

(fn SpawnLaneatSpawnPoint
  (params (isDark :type Boolean) (LaneNumber :type Integer))
  (CallFunction|SpawnLane (Transformation|GetWorldLocation (Variables|/Game/Blueprints/BP_Lane.BP_Lane_C|GetSpawnPoint (Variables|Default|GetNewestLane))) isDark LaneNumber))

(fn SpawnInitialLanes
  (for _index (range 0 4)
    (Utilities|IsValid (Variables|Default|GetNewestLane)
      (:Is%20Valid
        (CallFunction|SpawnLaneatSpawnPoint (Variables|/Game/Blueprints/BP_Lane.BP_Lane_C|GetisDark (Variables|Default|GetNewestLane))))
      (:Is%20Not%20Valid
        (CallFunction|SpawnLane (- (Transformation|GetActorLocation (Game|Player|GetPlayerPawn 0)) "700.000000,-500.000000,500.000000") true)))))