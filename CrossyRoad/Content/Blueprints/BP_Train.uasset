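; BP_Train is a train actor that moves endlessly along the world Y axis at a random speed and direction.
; The construction script stores its location as Anchor, rolls a non-zero signed Speed, and sets Anchor's Y to a fixed value for negative speeds.
; Tick adds Speed per frame without delta-time scaling, so movement is frame-rate dependent.
; Leaving the world Y bounds snaps it back to Anchor.
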(event EventBeginPlay)

(event Collision|EventActorBeginOverlap
  (params (OtherActor :type Actor%20Object%20Reference)))

(event EventTick
  (params (DeltaSeconds :type Float%20%28single-precision%29))
  (bind _returnvalue (Transformation|GetActorLocation))
  (Transformation|SetActorLocation (+ (Transformation|GetActorLocation) (Math|Vector|MakeVector 0.0 (Variables|Default|GetSpeed) 0.0)) false false)
  (if (or (< (.y _returnvalue) -1e+04) (> (.y _returnvalue) 1e+04))
    (Transformation|SetActorLocation (Variables|Default|GetAnchor) false false)))

(fn ConstructionScript
  (Variables|Default|SetAnchor (Transformation|GetActorLocation))
  (CallFunction|RandomizeSpeed)
  (if (< (Variables|Default|GetSpeed) 0.0)
    (Variables|Default|SetAnchor (Math|Vector|MakeVector (.x (Variables|Default|GetAnchor)) 4e+03 (.z (Variables|Default|GetAnchor))))))

(fn RandomizeSpeed
  (bind _output_get (Variables|Default|SetSpeed (Math|Random|RandomFloatinRange -1e+02 1e+02)))
  (if (== _output_get 0.0)
    (CallFunction|RandomizeSpeed)))